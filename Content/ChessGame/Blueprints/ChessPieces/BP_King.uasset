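; BP_King is the chess king piece, which highlights its possible moves on the board.
; ShowPossibleMoves clears highlights, then marks adjacent squares that are valid and not friend-occupied, without testing them for check.
; For an unmoved, uncastled king not in check, EvaluateCastlePath scans both ways along Y for an unmoved rook past empty squares.
; A found rook sets KingCanCastle, though the highlight is always at Y-2 because IsPositive is passed as false.
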(fn `EvaluateCastlePath`
  (params (YIncr :type Integer))
  (locals (CanContinue :type Boolean) (IsPositive :type Boolean) (TempY :type Integer))
  (bind (_chesspiece _isoccupied) (`/Game/ChessGame/Blueprints/BP_GameMode.GetOccupant` (`self.GameModeRef`) (`self.X`) (`local.TempY`) (`self.Color`)))
  (bind (_asbp_rook _bsuccess) (cast `/Game/ChessGame/Blueprints/ChessPieces/BP_Rook` _chesspiece :!pure true))
  (set `local.IsPositive` (> YIncr 0))
  (set `local.TempY` (`self.Y`))
  (set `local.CanContinue` true)
  (while (`local.CanContinue`)
    (set `local.TempY` (+ YIncr (`local.TempY`)))
    (if (and (< (`local.TempY`) 8) (> (`local.TempY`) 1))
      (set `local.CanContinue` (not (`.IsOccupied` (`/Game/ChessGame/Blueprints/BP_GameMode.GetOccupant` (`self.GameModeRef`) (`self.X`) (`local.TempY`) (`self.Color`)))))
      (elif (and _bsuccess _isoccupied)
        (if (`/Game/ChessGame/Blueprints/ChessPieces/BP_ChessPiece.IsInitialMove` _asbp_rook)
          (`self.HighlightCastleSquares` false)
          (set `local.CanContinue` false :!label _label))
        (else
          (goto _label))))))

(fn `EvaluateCastleSquares`
  (set `self.KingCanCastle` false)
  (if (not (`self.KingHasCastled`))
    (if (`self.IsInitialMove`)
      (if (not (`/Game/ChessGame/Blueprints/BP_GameMode.IsActiveKingInCheck` (`self.GameModeRef`)))
        (`|ExecutionSequence`
          (:`then_0`
            (`self.EvaluateCastlePath` 1))
          (:`then_1`
            (`self.EvaluateCastlePath` -1)))
        (else
          (set `self.KingCanCastle` false :!label _label)))
      (else
        (goto _label)))
    (else
      (goto _label))))

(fn `HighlightCastleSquares`
  (params (IsPositive :type Boolean))
  (locals (TempY :type Integer))
  (if IsPositive
    (bind _output_get (set `local.TempY` (+ (`self.Y`) 2)))
    (`self.HighlightPotentialSquares` (`self.X`) _output_get (`self.Color`))
    (set `self.KingCanCastle` true)
    (else
      (bind _output_get_2 (set `local.TempY` (+ (`self.Y`) -2)))
      (`self.HighlightPotentialSquares` (`self.X`) _output_get_2 (`self.Color`))
      (set `self.KingCanCastle` true))))

(fn `HighlightKingSquare`
  (params (XIncr :type Integer) (YIncr :type Integer))
  (locals (TempX :type Integer) (TempY :type Integer))
  (set `local.TempX` (+ (`self.X`) XIncr))
  (set `local.TempY` (+ (`self.Y`) YIncr))
  (if (`self.IsValidMoveForKing` (`local.TempX`) (`local.TempY`))
    (`self.HighlightPotentialSquares` (`local.TempX`) (`local.TempY`) (`self.Color`))))

(fn `IsValidMoveForKing`
  (params (X :type Integer) (Y :type Integer))
  (returns (IsValidMove :type Boolean))
  (bind (_chesspiece _isoccupied _isoccupiedbyfriend _isvalid) (`/Game/ChessGame/Blueprints/BP_GameMode.GetOccupant` (`self.GameModeRef`) X Y (`self.Color`)))
  (if _isvalid
    (if _isoccupiedbyfriend
      (return false)
      (else
        (return true)))
    (else
      (return false))))

(fn `ShowPossibleMoves`
  (returns (IsKing :type Boolean))
  (`|ExecutionSequence`
    (:`then_0`
      (`/Game/ChessGame/Blueprints/BP_GameMode.UnhighlightSquares` (`self.GameModeRef`))
      (set `self.KingCanCastle` false)
      (set `self.KingIsCastling` false))
    (:`then_1`
      (`self.HighlightKingSquare` 1)
      (`self.HighlightKingSquare` 1 1)
      (`self.HighlightKingSquare` 1 -1))
    (:`then_2`
      (`self.HighlightKingSquare` -1)
      (`self.HighlightKingSquare` -1 1)
      (`self.HighlightKingSquare` -1 -1))
    (:`then_3`
      (`self.HighlightKingSquare` 0 1)
      (`self.HighlightKingSquare` 0 -1))
    (:`then_4`
      (`self.EvaluateCastleSquares`)
      (return (`self.IsKing`)))))

(fn `UserConstructionScript`
  (`parent.UserConstructionScript`))